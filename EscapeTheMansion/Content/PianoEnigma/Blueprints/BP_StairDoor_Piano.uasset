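; Piano puzzle stair door that opens when piano buttons are pressed in the order stored in CodeArray.
; TurnPiano handles On signals by advancing a counter on each correct button, resetting it on a wrong one, printing it, and calling Open once the sequence completes.
; Two custom events play or reverse a timeline that scales the Stairs mesh along Z, with SoundControl switching sound on and, when finished, off.
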(event `CustomEvent`
  (`self.SoundControl` true)
  (bind (_direction _track) (`Timeline|Timeline` :!label _label)
    (:`Update`
      (`SceneComponent.SetWorldScale3D` (`self.Stairs`) (`KismetMathLibrary.MakeVector` 2.0 2.0 _track)))
    (:`Finished`
      (`self.SoundControl` false))))

(event `CustomEvent_1`
  (`self.SoundControl` true)
  (goto _label :!via `Reverse`))

(event `/Game/PianoEnigma/Blueprints/BI_Signal_Piano.TurnPiano`
  (params (Signal :type "/Game/FPSPuzzleSP/Blueprints/Components/Enum_Signal Enum" :default "NewEnumerator0") (NumButton :type Integer))
  (bind _countpiano (`self.CountPiano`))
  (bind _countpiano_2 (`self.CountPiano`))
  (switch `/Game/FPSPuzzleSP/Blueprints/Components/Enum_Signal` Signal
    (:`NewEnumerator0`
      (for (_array_element _array_index) (`self.CodeArray`)
        (bind _returnvalue (== _array_index _countpiano))
        (if _returnvalue
          (if (and (== NumButton _array_element) _returnvalue)
            (set `self.CountPiano` (+ _countpiano_2 1))
            (else
              (set `self.CountPiano` 0)))
          (`KismetSystemLibrary.PrintString` (`KismetStringLibrary.Conv_IntToString` _countpiano_2))
          (break)))
      (if (== _countpiano (`KismetArrayLibrary.Array_Length` (`self.CodeArray`)))
        (`self.Open`)))))

(fn `UserConstructionScript`
  (`parent.UserConstructionScript`))